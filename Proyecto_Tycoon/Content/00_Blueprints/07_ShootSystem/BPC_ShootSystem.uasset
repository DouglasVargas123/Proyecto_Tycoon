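; Actor component for the third-person character that handles axe equip and attack input along with melee hit detection.
; Input actions play draw, sheathe or downward attack montages based on AxeEquipped.
; While MeleAxe is true, Tick line-traces forward from the follow camera and notifies hit actors through BPI_Collision.
; AxeEquipped is only read here, and MeleAxe is only cleared, when attacking unequipped.
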(event `self.ReceiveBeginPlay`
  (bind _asbp_third_person_character (cast `/Game/00_Blueprints/00_ThirdPerson/Blueprints/BP_ThirdPersonCharacter` (`self.GetOwner`)))
  (set `self.Camera` (`/Game/00_Blueprints/00_ThirdPerson/Blueprints/BP_ThirdPersonCharacter.FollowCamera` _asbp_third_person_character))
  (set `self.As BP Third Person Character` _asbp_third_person_character))

(event `PreviewShoot`
  (bind (_returnvalue_location _returnvalue_rotation) (`KismetMathLibrary.BreakTransform` (`SceneComponent.K2_GetComponentToWorld` (`self.Camera`))))
  (bind (_outhit _returnvalue) (`KismetSystemLibrary.LineTraceSingle` _returnvalue_location (+ _returnvalue_location (* (`KismetMathLibrary.GetForwardVector` _returnvalue_rotation) (`self.ShootDistance`))) "TraceTypeQuery1"))
  (if _returnvalue
    (bind (_bblockinghit _binitialoverlap _time _distance _location _impactpoint _normal _impactnormal _physmat _hitactor) (`GameplayStatics.BreakHitResult` _outhit))
    (if (`KismetSystemLibrary.DoesImplementInterface` _hitactor "/Game/00_Blueprints/02_Blueprint_Interface/BPI_Collision.BPI_Collision_C")
      (message `/Game/00_Blueprints/02_Blueprint_Interface/BPI_Collision.On Collision Enter` _hitactor))))

(event `self.ReceiveTick`
  (params (DeltaSeconds :type "Float (single-precision)"))
  (if (`self.MeleAxe?`)
    (`self.PreviewShoot`)))

(event `EnhancedInput|/Game/00_Blueprints/00_ThirdPerson/Input/Actions/IA_AxeEquipped`
  (params (ActionValue :type Boolean) (ElapsedSeconds :type "Float (double-precision)") (TriggeredSeconds :type "Float (double-precision)") (InputAction :type "InputAction Object Reference" :default "/Game/00_Blueprints/00_ThirdPerson/Input/Actions/IA_AxeEquipped.IA_AxeEquipped"))
  (bind _mesh (`Character.Mesh` (`self.As BP Third Person Character`)))
  (:`Started`
    (if (`self.axeEquipped?`)
      (`|PlayMontage` _mesh "/Game/01_Models/Character2/Anim/Sheathing_Sword_Montage.Sheathing_Sword_Montage")
      (else
        (`|PlayMontage` _mesh "/Game/01_Models/Character2/Anim/Draw_Sword_1_Montage.Draw_Sword_1_Montage")))))

(event `EnhancedInput|/Game/00_Blueprints/00_ThirdPerson/Input/Actions/IA_AxeAttack`
  (params (ActionValue :type Boolean) (ElapsedSeconds :type "Float (double-precision)") (TriggeredSeconds :type "Float (double-precision)") (InputAction :type "InputAction Object Reference" :default "/Game/00_Blueprints/00_ThirdPerson/Input/Actions/IA_AxeAttack.IA_AxeAttack"))
  (:`Started`
    (if (`self.axeEquipped?`)
      (`|PlayMontage` (`Character.Mesh` (`self.As BP Third Person Character`)) "/Game/01_Models/Character2/Anim/Standing_Melee_Attack_Downward_Montage.Standing_Melee_Attack_Downward_Montage")
      (else
        (set `self.MeleAxe?` false)))))