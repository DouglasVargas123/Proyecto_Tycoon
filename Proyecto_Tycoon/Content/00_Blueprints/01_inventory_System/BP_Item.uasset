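; BP_Item is a world pickup that adds an item and quantity to the player's inventory.
; Its construction script looks up ItemInfo's data table row to set the mesh and the text label showing the item name.
; On collision, it casts player pawn 0 to BP_ThirdPersonCharacter without checking the colliding actor, calls AddToInventory on its BPInventoryComponent with the row name, then destroys itself.
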(event `/Game/00_Blueprints/02_Blueprint_Interface/BPI_Collision.On Collision Enter`
  (bind (_iteminfo_datatable _iteminfo_rowname) (break `DataTableRowHandle` (`self.ItemInfo`)))
  ;[1 1 1] Agregar al inventario
  (bind _asbp_third_person_character (cast `/Game/00_Blueprints/00_ThirdPerson/Blueprints/BP_ThirdPersonCharacter` (`GameplayStatics.GetPlayerPawn` 0)))
  (`/Game/00_Blueprints/01_inventory_System/BP_Inventory_Component.Add to inventory` (`/Game/00_Blueprints/00_ThirdPerson/Blueprints/BP_ThirdPersonCharacter.BP_Inventory_Component` _asbp_third_person_character) _iteminfo_rowname (`self.Quantity`))
  (`self.K2_DestroyActor` self))

(fn `UserConstructionScript`
  (bind (_iteminfo_datatable _iteminfo_rowname) (break `DataTableRowHandle` (`self.ItemInfo`)))
  (bind _returnvalue (`|GetDataTableRow` _iteminfo_datatable _iteminfo_rowname)
    (:`then`
      (bind (_nameitem _descriptionitem _buycost _sellcost _modelitem) (break `/Game/00_Blueprints/01_inventory_System/S_Item` _returnvalue))
      (`TextRenderComponent.K2_SetText` (`self.TextRender`) (`KismetTextLibrary.Conv_NameToText` _nameitem))
      (`StaticMeshComponent.SetStaticMesh` (`self.Item`) _modelitem))))