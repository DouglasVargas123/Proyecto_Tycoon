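; BP_Chest is an inventory-system chest that opens once and drops an item.
; Its collision-enter event sets Opened and plays the AbrirCofre timeline, which rolls the Scene component open.
; When the timeline finishes, it spawns a BP_Item at SpawnPoint, using either the configured ItemToDrop or, if IsRandom, a random row.
; Random row names come from ItemToDrop's data table, but the spawned item always references DT_Items.
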(event `/Game/00_Blueprints/02_Blueprint_Interface/BPI_Collision.On Collision Enter`
  (bind _itemtodrop_datatable (break `DataTableRowHandle` (`self.ItemToDrop`)))
  (if (not (`self.Opened?`))
    (set `self.Opened?` true)
    (bind (_direction _angle) (`Timeline|AbrirCofre`)
      (:`Update`
        (`SceneComponent.K2_SetRelativeRotation` (`self.Scene`) (`KismetMathLibrary.MakeRotator` _angle) false false))
      (:`Finished`
        (if (`self.isRandom`)
          (bind _outrownames (`DataTableFunctionLibrary.GetDataTableRowNames` _itemtodrop_datatable))
          (`|SpawnActorFromClass` "/Game/00_Blueprints/01_inventory_System/BP_Item.BP_Item_C" (`SceneComponent.K2_GetComponentToWorld` (`self.SpawnPoint`)) "Undefined" "MultiplyWithRoot" null (make `DataTableRowHandle` "/Game/00_Blueprints/01_inventory_System/DT_Items.DT_Items" (`|GetArrayItem` _outrownames (`KismetMathLibrary.RandomIntegerInRange` 0 (- (`KismetArrayLibrary.Array_Length` _outrownames) 1)))) null)
          (else
            (`|SpawnActorFromClass` "/Game/00_Blueprints/01_inventory_System/BP_Item.BP_Item_C" (`SceneComponent.K2_GetComponentToWorld` (`self.SpawnPoint`)) "Undefined" "MultiplyWithRoot" null (`self.ItemToDrop`) null)))))))

(fn `UserConstructionScript`)