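; Enemy character that roams random navmesh points, chases the player once Pawn Sensing spots them, and registers itself in the GameMode's enemy count.
; On reaching the player it plays a kick montage, then applies damage when the montage's duration elapses.
; Collision events reduce its health, spawning a coin on non-lethal hits or updating the GameMode count and destroying itself at zero.
; Tick refreshes its health bar widget.
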(event `self.ReceiveBeginPlay`
  ;[1 1 1] Third person cast
  (bind _asbp_third_person_character (cast `/Game/00_Blueprints/00_ThirdPerson/Blueprints/BP_ThirdPersonCharacter` (`GameplayStatics.GetPlayerPawn` 0)))
  (set `self.As BP Third Person Character` _asbp_third_person_character)
  (bind _asbp_third_person_game_mode (cast `/Game/00_Blueprints/00_ThirdPerson/Blueprints/BP_ThirdPersonGameMode` (`GameplayStatics.GetGameMode`)))
  (set `self.As BP Third Person Game Mode` _asbp_third_person_game_mode)
  (`/Engine/EditorBlueprintResources/StandardMacros.IncrementInt` (`/Game/00_Blueprints/00_ThirdPerson/Blueprints/BP_ThirdPersonGameMode.EnemyLeft` _asbp_third_person_game_mode)
    (:`  `
      (`self.RandomRoam`))))

(event `RandomRoam`
  ;[1 1 1] RANDOM WAPM
  (`|AIMoveTo` self (`NavigationSystemV1.K2_GetRandomReachablePointInRadius` (`self.K2_GetActorLocation`) 2500.0 null null) null
    (:`OnSuccess`
      (`self.RandomRoam`))))

(event `self.PawnSensing.OnSeePawn`
  (params (Pawn :type "Pawn Object Reference"))
  ;[1 1 1] Sens pawn
  (set `self.isSeeingPlayer` true)
  (`self.FollowPlayer`))

(event `FollowPlayer`
  ;[1 1 1] Sigue al jugador
  (set `self.canAttack` true)
  (if (`self.isSeeingPlayer`)
    (`|AIMoveTo` self (0.0 0.0 0.0) (`GameplayStatics.GetPlayerCharacter` 0) 50.0
      (:`OnSuccess`
        (if (`self.canAttack`)
          (set `self.canAttack` false)
          (bind _returnvalue (`self.PlayAnimMontage` "/Game/01_Models/06_NPC/AM_CharacterEnemyKick.AM_CharacterEnemyKick"))
          (`KismetSystemLibrary.Delay` _returnvalue)
          (bind _asbp_third_person_character (cast `/Game/00_Blueprints/00_ThirdPerson/Blueprints/BP_ThirdPersonCharacter` (`GameplayStatics.GetPlayerPawn` 0)))
          (`GameplayStatics.ApplyDamage` _asbp_third_person_character 1.0 null self)
          (set `self.canAttack` true))))))

(event `/Game/00_Blueprints/02_Blueprint_Interface/BPI_Collision.On Collision Enter`
  (bind _as_bp_third_person_game_mode (`self.As BP Third Person Game Mode`))
  ;[1 1 1] Collision player pega enemigo
  (bind _output_get (set `self.VidaActual` (- (`self.VidaActual`) 5.0)))
  (if (<= (`self.VidaActual`) 0.0)
    (`/Engine/EditorBlueprintResources/StandardMacros.DecrementInt` (`/Game/00_Blueprints/00_ThirdPerson/Blueprints/BP_ThirdPersonGameMode.EnemyLeft` _as_bp_third_person_game_mode)
      (:`  `
        (`/Game/00_Blueprints/00_ThirdPerson/Blueprints/BP_ThirdPersonGameMode.CheckEnemyLeft` _as_bp_third_person_game_mode)
        (`self.K2_DestroyActor`)))
    (else
      (`|SpawnActorFromClass` "/Game/00_Blueprints/10_Monedas/BP_Monedas1.BP_Monedas1_C" (`SceneComponent.K2_GetComponentToWorld` (`self.CapsuleComponent`)) "Undefined" "MultiplyWithRoot" null 0 null))))

(event `self.ReceiveTick`
  (params (DeltaSeconds :type "Float (single-precision)"))
  ;[1 1 1] EnemyuBar
  (bind _aswbp_enemy_health (cast `/Game/04_UI/WBP_EnemyHealth` (`WidgetComponent.GetWidget` (`self.HealthBarWidget`))))
  (`ProgressBar.SetPercent` (`/Game/04_UI/WBP_EnemyHealth.HealthEnemyBar` _aswbp_enemy_health) (/ (`self.VidaActual`) (`self.VidaMaxima`))))

(fn `CalcularVida`
  (bind _vidaactual (`self.VidaActual`))
  (set `self.VidaActual` (- 1.0 (`self.VidaActual`)))
  (if (<= _vidaactual 0.0)
    (`KismetSystemLibrary.PrintString` (`KismetStringLibrary.Conv_DoubleToString` _vidaactual))))

(fn `UserConstructionScript`)