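; BP_EnemySpawn is an enemy spawner that repeatedly creates waves of enemies at its own transform.
; On BeginPlay it spawns NumberOfEnemies of the Enemy class, waits SpawnDelay, then calls itself again in an endless loop.
; A backup spawn event creates BP_Enemy and grows an increment counter.
; A binding to the game mode's respawn event is left unconnected and never runs.
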(event `SpawnEnemy`
  ;[1 1 1] Por si acaso
  (for _ (range (`self.EnemySpawned`))
    (`|SpawnActorFromClass` "/Game/00_Blueprints/05_Enemy/BP_Enemy.BP_Enemy_C" (`self.GetTransform`) "Undefined" "MultiplyWithRoot" null null))
  (`/Engine/EditorBlueprintResources/StandardMacros.IncrementInt` (`self.EnemyIncrement`)
    (:`  `
      (set `self.EnemyIncrement` (+ (`self.EnemySpawned`) (`self.EnemyIncrement`))))))

(event `self.ReceiveBeginPlay`
  (`self.Spawn Enemy` (`self.Enemy`) (`self.GetTransform`) (`self.NumberOfEnemies`)))

(event `Spawn Enemy`
  (params (Enemy :type "Actor Class Reference") (SpawnTransform :type "Transform Structure") (NumberOfEnemies :type Integer))
  (for _ (range NumberOfEnemies)
    (`|SpawnActorFromClass` Enemy SpawnTransform "Undefined" "MultiplyWithRoot" null null))
  (`KismetSystemLibrary.Delay` (`self.SpawnDelay`))
  (`self.Spawn Enemy` (`self.Enemy`) (`self.GetTransform`) (`self.NumberOfEnemies`)))

(fn `UserConstructionScript`)