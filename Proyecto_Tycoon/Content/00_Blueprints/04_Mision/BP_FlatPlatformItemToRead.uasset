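; Flat platform actor that sells a valuable object for 50 coins, spawning it at the PostToBuild transform.
; On BeginPlay it caches DT_Objetos_De_Valor rows; on collision it deducts the fixed price from the GameMode's MonedasTotal and spawns the actor at Index.
; The construction script shows PalabraArriba on a text render.
; An inventory-for-building exchange is left disconnected, and each row's Valor is unused.
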(event `self.ReceiveBeginPlay`
  (bind _outrownames (`DataTableFunctionLibrary.GetDataTableRowNames` "/Game/00_Blueprints/10_Monedas/Database/DT_Objetos_De_Valor.DT_Objetos_De_Valor"))
  (for _array_element _outrownames
    (bind _returnvalue (`|GetDataTableRow` "/Game/00_Blueprints/10_Monedas/Database/DT_Objetos_De_Valor.DT_Objetos_De_Valor" _array_element)
      (:`then`
        (`KismetArrayLibrary.Array_Add` (`self.ObjetosDeValor`) _returnvalue)))))

(event `/Game/00_Blueprints/02_Blueprint_Interface/BPI_Collision.On Collision Enter`
  ;[1 1 1] cOLLISON
  (bind _asbp_third_person_game_mode (cast `/Game/00_Blueprints/00_ThirdPerson/Blueprints/BP_ThirdPersonGameMode` (`GameplayStatics.GetGameMode`)))
  (if (>= (`/Game/00_Blueprints/00_ThirdPerson/Blueprints/BP_ThirdPersonGameMode.MonedasTotal` _asbp_third_person_game_mode) 50)
    (set `/Game/00_Blueprints/00_ThirdPerson/Blueprints/BP_ThirdPersonGameMode.MonedasTotal` (- (`/Game/00_Blueprints/00_ThirdPerson/Blueprints/BP_ThirdPersonGameMode.MonedasTotal` _asbp_third_person_game_mode) 50) _asbp_third_person_game_mode)
    (`|SpawnActorFromClass` (`.Actor_10_DACDE3E249FB87C0B19FA2B29F838D1E` (break `/Game/00_Blueprints/10_Monedas/Database/S_Monedas` (`|GetArrayItem` (`self.ObjetosDeValor`) (`self.Index`)))) (`self.GetTransform` (`self.PostToBuild`)) "Undefined" "MultiplyWithRoot" null null)))

(fn `UserConstructionScript`
  (`TextRenderComponent.K2_SetText` (`self.TextRender1`) (`KismetTextLibrary.Conv_StringToText` (`self.PalabraArriba`))))