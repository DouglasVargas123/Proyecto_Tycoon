(event `self.ReceiveBeginPlay`
  ;[1 1 1] Ref
  (`|ExecutionSequence`
    (:`then_0`
      (bind _asbp_third_person_character (cast `/Game/00_Blueprints/00_ThirdPerson/Blueprints/BP_ThirdPersonCharacter` (`self.GetOwner`)))
      (set `self.Camera` (`/Game/00_Blueprints/00_ThirdPerson/Blueprints/BP_ThirdPersonCharacter.FollowCamera` _asbp_third_person_character))
      (set `self.BP_Character` _asbp_third_person_character)
      (bind _outrownames (`DataTableFunctionLibrary.GetDataTableRowNames` "/Game/00_Blueprints/06_BuildingSystem/DataBase/DT_BuildParts.DT_BuildParts"))
      (for _array_element _outrownames
        (bind _returnvalue (`|GetDataTableRow` "/Game/00_Blueprints/06_BuildingSystem/DataBase/DT_BuildParts.DT_BuildParts" _array_element)
          (:`then`
            (`KismetArrayLibrary.Array_Add` (`self.DT_Buidables`) _returnvalue)))))
    (:`then_1`
      (bind _asbp_third_person_game_mode (cast `/Game/00_Blueprints/00_ThirdPerson/Blueprints/BP_ThirdPersonGameMode` (`GameplayStatics.GetGameMode`)))
      (set `self.GM` _asbp_third_person_game_mode))))

(event `PreviewLook`
  (bind (_returnvalue_location _returnvalue_rotation) (`KismetMathLibrary.BreakTransform` (`SceneComponent.K2_GetComponentToWorld` (`self.Camera`))))
  ;[1 1 1] Raycast
  (bind (_outhit _returnvalue) (`KismetSystemLibrary.LineTraceSingle` _returnvalue_location (+ _returnvalue_location (* (`KismetMathLibrary.GetForwardVector` _returnvalue_rotation) (`self.BuildDistance`))) "TraceTypeQuery1"))
  (if _returnvalue
    (`|ExecutionSequence`
      (:`then_0`
        (`/Engine/EditorBlueprintResources/StandardMacros.DoOnce` false :!label _label
          (:`Completed`
            (bind _returnvalue_2 (`|AddComponentByClass` (`self.BP_Character`) "/Script/Engine.StaticMeshComponent" false (`self.BuildPreviewTransform`)))
            (bind _output_get (set `self.PreviewMesh` _returnvalue_2))
            (`StaticMeshComponent.SetStaticMesh` _output_get (`.Mesh_6_1E58E4314B6CA628E4EBC09F96E466A1` (break `/Game/00_Blueprints/06_BuildingSystem/DataBase/S_BuildParts` (`|GetArrayItem` (`self.DT_Buidables`) (`self.Buildable_Index`)))))
            (`PrimitiveComponent.SetMaterial` (`self.PreviewMesh`) 0 "/Game/02_Material/MaterialPreview/M_BuildingPreview.M_BuildingPreview")
            (`PrimitiveComponent.SetCollisionEnabled` (`self.PreviewMesh`) "NoCollision"))))
      (:`then_1`
        (bind _output_get_2 (set `self.BuildPreviewTransform` (`KismetMathLibrary.MakeTransform` (`.Location` (`GameplayStatics.BreakHitResult` _outhit)) (`self.Build Preview Rotation`) (5.0 5.0 5.0))))
        (`SceneComponent.K2_SetWorldTransform` (`self.PreviewMesh`) _output_get_2 false false)))))

(event `ResetBuildMode`
  ;[1 1 1] Raycast
  (goto _label :!via `Reset`))

(event `EnhancedInput|/Game/00_Blueprints/00_ThirdPerson/Input/Actions/IA_PlaceBuilding`
  (params (ActionValue :type Boolean) (ElapsedSeconds :type "Float (double-precision)") (TriggeredSeconds :type "Float (double-precision)") (InputAction :type "InputAction Object Reference" :default "/Game/00_Blueprints/00_ThirdPerson/Input/Actions/IA_PlaceBuilding.IA_PlaceBuilding"))
  (bind _cantidad_madera (`/Game/00_Blueprints/00_ThirdPerson/Blueprints/BP_ThirdPersonGameMode.Cantidad Madera` (`self.GM`)))
  ;[1 1 1] Colocar contruccion
  (:`Started`
    (if (>= _cantidad_madera 1)
      (`/Engine/EditorBlueprintResources/StandardMacros.DecrementInt` _cantidad_madera
        (:`  `
          (if (`self.inBuildMode?`)
            (bind _result (`/Engine/EditorBlueprintResources/StandardMacros.IncrementInt` (`/Game/00_Blueprints/00_ThirdPerson/Blueprints/BP_ThirdPersonGameMode.ObjetosConstruidos` (`self.GM`)))
              (:`  `
                (`KismetSystemLibrary.PrintString` (`KismetStringLibrary.Conv_IntToString` _result))
                (`|SpawnActorFromClass` (`.Blueprint_9_52EBC13C4A8332E0D5BFF5801FA2EAD5` (break `/Game/00_Blueprints/06_BuildingSystem/DataBase/S_BuildParts` (`|GetArrayItem` (`self.DT_Buidables`) (`self.Buildable_Index`)))) (`self.BuildPreviewTransform`) "Undefined" "MultiplyWithRoot" null null)
                (`self.Stop Build Mode`)))))))))

(event `self.ReceiveTick`
  (params (DeltaSeconds :type "Float (single-precision)"))
  ;[1 1 1] Preview loop
  (if (`self.inBuildMode?`)
    (`self.PreviewLook`)))

(event `EnhancedInput|/Game/00_Blueprints/00_ThirdPerson/Input/Actions/IA_Build`
  (params (ActionValue :type Boolean) (ElapsedSeconds :type "Float (double-precision)") (TriggeredSeconds :type "Float (double-precision)") (InputAction :type "InputAction Object Reference" :default "/Game/00_Blueprints/00_ThirdPerson/Input/Actions/IA_Build.IA_Build"))
  ;[1 1 1] Construir
  (:`Started`
    (if (not (`self.inBuildMode?`))
      (set `self.inBuildMode?` true)
      (else
        (set `self.inBuildMode?` false :!label _label_2)
        (bind _previewmesh (`self.PreviewMesh`)
          (:`then`
            (`StaticMeshComponent.SetStaticMesh` _previewmesh null)
            (set `self.PreviewMesh` null)
            (`self.ResetBuildMode`))
          (:`else`))))))

(event `Stop Build Mode`
  ;[1 1 1] Construir
  (goto _label_2))

(event `EnhancedInput|/Game/00_Blueprints/00_ThirdPerson/Input/Actions/IA_BuildRotation`
  (params (ActionValue :type Boolean) (ElapsedSeconds :type "Float (double-precision)") (TriggeredSeconds :type "Float (double-precision)") (InputAction :type "InputAction Object Reference" :default "/Game/00_Blueprints/00_ThirdPerson/Input/Actions/IA_BuildRotation.IA_BuildRotation"))
  ;[1 1 1] Rotar
  (:`Started`
    (bind _returnvalue (`KismetSystemLibrary.K2_SetTimerDelegate` (delegate `Rotate Preview`) 0.1 true))
    (set `self.Rotate Preview Loop` _returnvalue))
  (:`Completed`
    (`KismetSystemLibrary.K2_ClearAndInvalidateTimerHandle` (`self.Rotate Preview Loop`))
    (set `self.Rotate Preview Loop` (struct))))

(event `Rotate Preview`
  (bind (_buildpreviewtransform_location _buildpreviewtransform_rotation) (`KismetMathLibrary.BreakTransform` (`self.BuildPreviewTransform`)))
  ;[1 1 1] Rotar
  (set `self.Build Preview Rotation` (`KismetMathLibrary.ComposeRotators` _buildpreviewtransform_rotation (struct :`Yaw` 5.0))))

(event `Key|MouseScrollUp`
  (params (Key :type "Key Structure"))
  ;[1 1 1] Pasar por objetos
  (:`Pressed`
    (set `self.Buildable_Index` (`KismetMathLibrary.Clamp` (+ (`self.Buildable_Index`) 1) 0 (- (`KismetArrayLibrary.Array_Length` (`self.DT_Buidables`)) 1)))
    (bind _previewmesh (`self.PreviewMesh` :!label _label_3)
      (:`then`
        (`StaticMeshComponent.SetStaticMesh` _previewmesh null)
        (set `self.PreviewMesh` null)
        (`self.ResetBuildMode`))
      (:`else`))))

(event `Key|MouseScrollDown`
  (params (Key :type "Key Structure"))
  ;[1 1 1] Pasar por objetos
  (:`Pressed`
    (set `self.Buildable_Index` (`KismetMathLibrary.Clamp` (- (`self.Buildable_Index`) 1) 0 (- (`KismetArrayLibrary.Array_Length` (`self.DT_Buidables`)) 1)))
    (goto _label_3)))

(event `EnhancedInput|/Game/00_Blueprints/00_ThirdPerson/Input/Actions/IA_Destroy`
  (params (ActionValue :type Boolean) (ElapsedSeconds :type "Float (double-precision)") (TriggeredSeconds :type "Float (double-precision)") (InputAction :type "InputAction Object Reference" :default "/Game/00_Blueprints/00_ThirdPerson/Input/Actions/IA_Destroy.IA_Destroy"))
  (bind (_returnvalue_location _returnvalue_rotation) (`KismetMathLibrary.BreakTransform` (`SceneComponent.K2_GetComponentToWorld` (`self.Camera`))))
  ;[1 1 1] Destruir
  (:`Started`
    (bind (_outhit _returnvalue) (`KismetSystemLibrary.LineTraceSingle` _returnvalue_location (+ _returnvalue_location (* (`KismetMathLibrary.GetForwardVector` _returnvalue_rotation) (`self.BuildDistance`))) "TraceTypeQuery1"))
    (if _returnvalue
      (bind (_bblockinghit _binitialoverlap _time _distance _location _impactpoint _normal _impactnormal _physmat _hitactor) (`GameplayStatics.BreakHitResult` _outhit))
      (if (`Actor.ActorHasTag` _hitactor "Buildable")
        (`Actor.K2_DestroyActor` _hitactor)))))