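; BP_MasterMadera is a wood (madera) resource actor, likely the base for wood pickups, that adds to the wood count when touched.
; BeginPlay caches a reference to BP_ThirdPersonGameMode, which holds the CantidadMadera counter.
; OnCollisionEnter increments that counter without checking what collided, prints the new total, then destroys the actor after a short delay.
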(event `self.ReceiveBeginPlay`
  ;[0 0 0] GM_Ref
  (bind _asbp_third_person_game_mode (cast `/Game/00_Blueprints/00_ThirdPerson/Blueprints/BP_ThirdPersonGameMode` (`GameplayStatics.GetGameMode`)))
  (set `self.GMRef` _asbp_third_person_game_mode))

(event `/Game/00_Blueprints/02_Blueprint_Interface/BPI_Collision.On Collision Enter`
  (bind _gmref (`self.GMRef`))
  (bind _cantidad_madera (`/Game/00_Blueprints/00_ThirdPerson/Blueprints/BP_ThirdPersonGameMode.Cantidad Madera` _gmref))
  ;[1 1 1] Collision
  (bind _result (`/Engine/EditorBlueprintResources/StandardMacros.IncrementInt` _cantidad_madera)
    (:`  `
      (set `/Game/00_Blueprints/00_ThirdPerson/Blueprints/BP_ThirdPersonGameMode.Cantidad Madera` _result _gmref)
      (`KismetSystemLibrary.PrintString` (`KismetStringLibrary.Conv_IntToString` _cantidad_madera))
      (`KismetSystemLibrary.Delay` 0.2)
      (`self.K2_DestroyActor`))))

(fn `UserConstructionScript`)