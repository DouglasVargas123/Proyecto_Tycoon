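; Base tree Blueprint that loses health on each collision-enter event and drops an item when destroyed.
; At zero health it destroys its static mesh and spawns a BP_Item at the Scene component's transform.
; The IsRandom flag selects between a random DT_Items row, named from DataTableRow's table, and the configured DataTableRow, which spawns after a short delay.
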(event `/Game/00_Blueprints/02_Blueprint_Interface/BPI_Collision.On Collision Enter`
  (bind _data_table_row_datatable (break `DataTableRowHandle` (`self.Data Table Row`)))
  (bind _result (`/Engine/EditorBlueprintResources/StandardMacros.DecrementFloat` (`self.vidaActual`))
    (:`  `
      (set `self.vidaActual` _result)
      (if (<= (`self.vidaActual`) 0.0)
        (`ActorComponent.K2_DestroyComponent` (`self.StaticMesh`))
        (if (not (`self.isRandom?`))
          (`KismetSystemLibrary.Delay` 0.5)
          (`|SpawnActorFromClass` "/Game/00_Blueprints/01_inventory_System/BP_Item.BP_Item_C" (`SceneComponent.K2_GetComponentToWorld` (`self.Scene`)) "Undefined" "MultiplyWithRoot" null (`self.Data Table Row`) null)
          (else
            (bind _outrownames (`DataTableFunctionLibrary.GetDataTableRowNames` _data_table_row_datatable))
            (`|SpawnActorFromClass` "/Game/00_Blueprints/01_inventory_System/BP_Item.BP_Item_C" (`SceneComponent.K2_GetComponentToWorld` (`self.Scene`)) "Undefined" "MultiplyWithRoot" null (make `DataTableRowHandle` "/Game/00_Blueprints/01_inventory_System/DT_Items.DT_Items" (`|GetArrayItem` _outrownames (`KismetMathLibrary.RandomIntegerInRange` 0 (- (`KismetArrayLibrary.Array_Length` _outrownames) 1)))) null)))))))

(fn `UserConstructionScript`)